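; BP_Player is a mouse-driven player Blueprint that places characters on spawn areas and moves its camera.
; Two input actions trace from the cursor and spawn a scaled BP_Al or BP_Muffin where the hit actor is a BP_SpawnArea.
; The CameraMovement axis restarts a timeline whose output, times the axis value, feeds DeplaceCamera.
; That function slides the camera along its forward vector, scaling each step by its distance to the root.
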(event `self.ReceiveBeginPlay`
  (set `PlayerController.bShowMouseCursor` true (`GameplayStatics.GetPlayerController` 0)))

(event `InputAction|SpawnAlCapone`
  (params (Key :type "Key Structure"))
  (bind (_worldlocation _worlddirection) (`PlayerController.DeprojectMousePositionToWorld` (`GameplayStatics.GetPlayerController` 0)))
  (:`Pressed`
    (bind _outhit (`KismetSystemLibrary.LineTraceSingle` _worldlocation (+ _worldlocation (* _worlddirection (`self.TraceDistance`))) "TraceTypeQuery1"))
    (bind (_bblockinghit _binitialoverlap _time _distance _location _impactpoint _normal _impactnormal _physmat _hitactor) (`GameplayStatics.BreakHitResult` _outhit))
    (cast `/Game/CreationTP9/Blueprints/BP_SpawnArea` _hitactor)
    (`|SpawnActorFromClass` "/Game/CreationTP9/Characters/AlcaponeVoxels/BluePrints/BP_Al.BP_Al_C" (`KismetMathLibrary.MakeTransform` _location (struct) (8.0 8.0 8.0)) "AdjustIfPossibleButAlwaysSpawn" "OverrideRootScale" null null)))

(event `InputAction|SpawnMuffin`
  (params (Key :type "Key Structure"))
  (bind (_worldlocation _worlddirection) (`PlayerController.DeprojectMousePositionToWorld` (`GameplayStatics.GetPlayerController` 0)))
  (:`Pressed`
    (bind _outhit (`KismetSystemLibrary.LineTraceSingle` _worldlocation (+ _worldlocation (* _worlddirection (`self.TraceDistance`))) "TraceTypeQuery1"))
    (bind (_bblockinghit _binitialoverlap _time _distance _location _impactpoint _normal _impactnormal _physmat _hitactor) (`GameplayStatics.BreakHitResult` _outhit))
    (cast `/Game/CreationTP9/Blueprints/BP_SpawnArea` _hitactor)
    (`|SpawnActorFromClass` "/Game/CreationTP9/Characters/Muffin/Blueprints/BP_Muffin.BP_Muffin_C" (`KismetMathLibrary.MakeTransform` _location (struct) (2.0 2.0 2.0)) "AdjustIfPossibleButAlwaysSpawn" "OverrideRootScale" null null)))

(event `InputAxis|CameraMovement`
  (params (AxisValue :type "Float (single-precision)"))
  (bind (_direction _t) (`Timeline|Timeline_0` :!via `PlayFromStart`)
    (:`Update`
      (`self.deplaceCamera` (* AxisValue _t)))))

(fn `deplaceCamera`
  (params (distance :type "Float (double-precision)"))
  (`SceneComponent.K2_SetRelativeLocation` (`self.Camera`) (+ (* (`KismetMathLibrary.GetForwardVector` (`SceneComponent.RelativeRotation` (`self.Camera`))) (* distance (`KismetMathLibrary.VSize` (- (`SceneComponent.RelativeLocation` (`self.DefaultSceneRoot`)) (`SceneComponent.RelativeLocation` (`self.Camera`)))))) (`SceneComponent.RelativeLocation` (`self.Camera`))) false false))

(fn `UserConstructionScript`)